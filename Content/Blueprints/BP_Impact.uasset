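; BP_Impact is a short-lived impact effect actor built from two widget components.
; On BeginPlay it turns both widgets once toward the player camera, then scatters each by a random world offset.
; A timeline drives their uniform scale between zero and a small size, and the actor destroys itself after a brief delay when it finishes.
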(event `self.ReceiveBeginPlay`
  (bind _returnvalue (`KismetMathLibrary.RandomFloatInRange` -50.0 50.0))
  (bind _returnvalue_2 (`KismetMathLibrary.RandomFloatInRange` -30.0 30.0))
  (bind _returnvalue_3 (`KismetMathLibrary.RandomFloatInRange` -30.0 30.0))
  (bind _returnvalue_4 (`PlayerCameraManager.GetCameraLocation` (`GameplayStatics.GetPlayerCameraManager` 0)))
  (`SceneComponent.K2_SetWorldRotation` (`self.Widget 1`) (`KismetMathLibrary.FindLookAtRotation` (`SceneComponent.K2_GetComponentLocation` (`self.Widget 1`)) _returnvalue_4) false false)
  (`SceneComponent.K2_SetWorldRotation` (`self.Widget 2`) (`KismetMathLibrary.FindLookAtRotation` (`SceneComponent.K2_GetComponentLocation` (`self.Widget 2`)) _returnvalue_4) false false)
  (`SceneComponent.K2_AddWorldOffset` (`self.Widget 1`) (`KismetMathLibrary.MakeVector` _returnvalue_2 _returnvalue_3 _returnvalue) false false)
  (`SceneComponent.K2_AddWorldOffset` (`self.Widget 2`) (`KismetMathLibrary.MakeVector` _returnvalue_2 _returnvalue_3 _returnvalue) false false)
  (bind (_direction _newtrack_1) (`Timeline|Scale Timeline` :!via `PlayFromStart`)
    (:`Update`
      (bind _returnvalue_5 (`KismetMathLibrary.Conv_DoubleToVector` (`KismetMathLibrary.Lerp` 0.0 0.1 _newtrack_1)))
      (`SceneComponent.SetRelativeScale3D` (`self.Widget 1`) _returnvalue_5)
      (`SceneComponent.SetRelativeScale3D` (`self.Widget 2`) _returnvalue_5))
    (:`Finished`
      (`KismetSystemLibrary.Delay` 0.2)
      (`self.K2_DestroyActor`))))

(event `self.ReceiveTick`
  (params (DeltaSeconds :type "Float (single-precision)")))

(fn `UserConstructionScript`)